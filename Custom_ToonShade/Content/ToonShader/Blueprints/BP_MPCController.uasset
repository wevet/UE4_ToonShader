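; BP_MPCController is an actor that drives the toon shader's global look through the MPC_Toon Material Parameter Collection.
; UpdateParams copies the actor's ambient, base color, base-color-to-emissive and unlit intensity variables into the collection's scalar parameters.
; It runs from the Construction Script for updates in the editor and again every Tick, so changes apply continuously at runtime.
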(event `self.ReceiveTick`
  (params (DeltaSeconds :type "Float (single-precision)"))
  (`self.UpdateParams`))

(fn `UpdateParams`
  (`KismetMaterialLibrary.SetScalarParameterValue` "/Game/ToonShader/Materials/MPC_Toon.MPC_Toon" "AmbientIntencity" (`self.AmbientIntensity`))
  (`KismetMaterialLibrary.SetScalarParameterValue` "/Game/ToonShader/Materials/MPC_Toon.MPC_Toon" "BaseColorAddtoEmissiveScale" (`self.BaseColorAddToEmissiveScale`))
  (`KismetMaterialLibrary.SetScalarParameterValue` "/Game/ToonShader/Materials/MPC_Toon.MPC_Toon" "BaseColorScale" (`self.BaseColorScale`))
  (`KismetMaterialLibrary.SetScalarParameterValue` "/Game/ToonShader/Materials/MPC_Toon.MPC_Toon" "UnlitIntensity" (`self.UnlitIntensity`)))

(fn `UserConstructionScript`
  (`self.UpdateParams`))