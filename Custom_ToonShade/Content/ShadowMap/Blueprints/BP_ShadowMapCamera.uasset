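; Orthographic scene-capture camera for a custom shadow map, viewing the scene along the first directional light's direction.
; Each tick it snaps to a fixed distance back from world origin along that light's forward vector.
; It writes its location, axes and ortho width to MPC_ShadowMap as light-view data for materials.
; It also rescans all actors every tick, setting Pawns as show-only and others as hidden.
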(event `self.ReceiveBeginPlay`
  (bind _othrowidth (`self.OthroWidth`))
  (set `SceneCaptureComponent2D.OrthoWidth` _othrowidth (`self.SceneCaptureComponent2D`))
  (`KismetMaterialLibrary.SetScalarParameterValue` "/Game/ShadowMap/Materials/MPC_ShadowMap.MPC_ShadowMap" "ShadowOthroWidth" _othrowidth)
  (`self.SetLightActor`))

(event `self.ReceiveTick`
  (params (DeltaSeconds :type "Float (single-precision)"))
  (`self.UpdateMaterialParamaters`)
  (`self.UpdateCaptureActors`))

(fn `SetLightActor`
  (bind _outactors (`GameplayStatics.GetAllActorsOfClass` "/Script/Engine.DirectionalLight"))
  (if (> (`KismetArrayLibrary.Array_Length` _outactors) 0)
    (set `self.LightActor` (`|GetArrayItem` _outactors))))

(fn `UpdateCaptureActors`
  (locals (PawnArray :type "Array of Pawn Object Reference") (ActorArray :type "Array of Actor Object Reference"))
  (bind _scenecapturecomponent2d (`self.SceneCaptureComponent2D`))
  (bind _outactors (`GameplayStatics.GetAllActorsOfClass` "/Script/Engine.Actor"))
  (for _array_element _outactors
    (if (not (== _array_element self))
      (bind (_aspawn _bsuccess) (cast `Pawn` _array_element :!pure true))
      (if _bsuccess
        (`KismetArrayLibrary.Array_Add` (`local.PawnArray`) _aspawn)
        (else
          (`KismetArrayLibrary.Array_Add` (`local.ActorArray`) _array_element)))))
  (set `SceneCaptureComponent.ShowOnlyActors` (`local.PawnArray`) _scenecapturecomponent2d)
  (set `SceneCaptureComponent.HiddenActors` (`local.ActorArray`) _scenecapturecomponent2d))

(fn `UpdateMaterialParamaters`
  (locals (CaptureTransform :type "Transform Structure"))
  (bind _lightactor (`self.LightActor`))
  (bind _rotation (.rotation (`local.CaptureTransform`)))
  (if (`KismetSystemLibrary.IsValid` _lightactor)
    (bind _output_get (set `local.CaptureTransform` (`KismetMathLibrary.MakeTransform` (* (`self.GetActorForwardVector` _lightactor) -10000.0) (`self.K2_GetActorRotation` _lightactor))))
    (`self.K2_SetActorTransform` _output_get false true)
    (`KismetMaterialLibrary.SetVectorParameterValue` "/Game/ShadowMap/Materials/MPC_ShadowMap.MPC_ShadowMap" "CaptureLocation" (`KismetMathLibrary.Conv_VectorToLinearColor` (.location (`local.CaptureTransform`))))
    (`KismetMaterialLibrary.SetVectorParameterValue` "/Game/ShadowMap/Materials/MPC_ShadowMap.MPC_ShadowMap" "LightViewMatrixPlaneX" (`KismetMathLibrary.Conv_VectorToLinearColor` (`KismetMathLibrary.GetRightVector` _rotation)))
    (`KismetMaterialLibrary.SetVectorParameterValue` "/Game/ShadowMap/Materials/MPC_ShadowMap.MPC_ShadowMap" "LightViewMatrixPlaneY" (`KismetMathLibrary.Conv_VectorToLinearColor` (`KismetMathLibrary.GetUpVector` _rotation)))
    (`KismetMaterialLibrary.SetVectorParameterValue` "/Game/ShadowMap/Materials/MPC_ShadowMap.MPC_ShadowMap" "LightViewMatrixPlaneZ" (`KismetMathLibrary.Conv_VectorToLinearColor` (`KismetMathLibrary.GetForwardVector` _rotation)))))

(fn `UserConstructionScript`)